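; MainGameState watches the player's lives and shows the lose screen when they run out.
; Every Tick it casts the first player pawn to BattleBumperPlayer_BlueprintNight and reads its lives.
; At zero it adds WP_LoseScreen to the viewport, with a Lost flag so this happens only once.
; Win-screen creation and a camera blend to the player's PlayerAssasin camera owner are present but unwired.
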(event EventBeginPlay)

(event EventTick
  (params (DeltaSeconds :type Float%20%28single-precision%29))
  (bind _asbattle_bumper_player_blueprint_night (Utilities|Casting|CastToBattleBumperPlayer_BlueprintNight (Game|Player|GetPlayerPawn 0)))
  (bind _returnvalue (Class|MyPlayerState|ReturnPlayerLives _asbattle_bumper_player_blueprint_night))
  (Math|Integer|CompareInt _returnvalue
    (:==
      (if (not (Variables|Default|GetLost))
        (bind _returnvalue_2 (UserInterface|CreateWidget "/Game/Widgets/WP_LoseScreen.WP_LoseScreen_C" (Game|GetPlayerController 0)))
        (UserInterface|Viewport|AddtoViewport _returnvalue_2 0)
        (Variables|Default|SetLost true)))))

(fn ConstructionScript)